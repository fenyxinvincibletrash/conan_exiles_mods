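; Two-handed light bow weapon that handles bowstring animation and the arrow shown in the archer's hand.
; Character signals for draw, loop, fire and settle play string animations on the weapon mesh, with first/third-person branches mostly sharing assets.
; The animation blueprint's pick-arrow signal spawns a non-replicated visual projectile using the active ammo's mesh, skipped on the server for remote actors.
; That arrow is destroyed on combat exit and EndPlay.
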(event Custom|SignalSecondaryStringLoop
  (if (Variables|Default|GetInThirdPerson)
    (Components|Animation|PlayAnimation (Variables|Default|GetWeaponSkeletalMesh) "/Game/Items/Weapons/Bow/Animations/A_combat_bow_string_heavy_loop.A_combat_bow_string_heavy_loop" false)
    (else
      (Components|Animation|PlayAnimation (Variables|Default|GetWeaponSkeletalMesh) "/Game/Items/Weapons/Bow/Animations/A_combat_bow_string_heavy_loop.A_combat_bow_string_heavy_loop" false))))

(event Custom|SignalSecondaryStringSettle
  ;[1 1 1] Basic String Settle
  (if (Variables|Default|GetInThirdPerson)
    (Components|Animation|PlayAnimation (Variables|Default|GetWeaponSkeletalMesh) "/Game/Items/Weapons/Bow/Animations/A_bow_3rd_secondary_special_settle.A_bow_3rd_secondary_special_settle" false)
    (else
      (Components|Animation|PlayAnimation (Variables|Default|GetWeaponSkeletalMesh) "/Game/Items/Weapons/Bow/Animations/A_bow_3rd_secondary_special_settle.A_bow_3rd_secondary_special_settle" false))))

(event Custom|SignalBowStringExecute
  (params (Source :type E_AttackSource%20Enum))
  ;[1 1 1] Basic String Execute
  (if (Utilities|Enum|Equal(Enum) Source "NewEnumerator4")
    (if (Variables|Default|GetInThirdPerson)
      (Components|Animation|PlayAnimation (Variables|Default|GetWeaponSkeletalMesh) "/Game/Items/Weapons/Bow/Animations/A_combat_bow_string_heavy_fire.A_combat_bow_string_heavy_fire" false)
      (else
        (Components|Animation|PlayAnimation (Variables|Default|GetWeaponSkeletalMesh) "/Game/Items/Weapons/Bow/Animations/A_combat_bow_string_heavy_fire.A_combat_bow_string_heavy_fire" false)))))

(event Custom|SignalSecondaryStringDraw
  ;[1 1 1] Basic String Draw
  (if (Variables|Default|GetInThirdPerson)
    (Components|Animation|PlayAnimation (Variables|Default|GetWeaponSkeletalMesh) "/Game/Items/Weapons/Bow/Animations/A_combat_bow_string_heavy_charge.A_combat_bow_string_heavy_charge" false)
    (else
      (Components|Animation|PlayAnimation (Variables|Default|GetWeaponSkeletalMesh) "/Game/Items/Weapons/Bow/Animations/A_combat_bow_string_heavy_charge.A_combat_bow_string_heavy_charge" false))))

(event Custom|SignalPrimaryStringDraw
  ;[1 1 1] Basic String Draw
  (if (Variables|Default|GetInThirdPerson)
    (Components|Animation|PlayAnimation (Variables|Default|GetWeaponSkeletalMesh) "/Game/Items/Weapons/Bow/Animations/A_bow_3rd_draw_c2.A_bow_3rd_draw_c2" false)
    (else
      (Components|Animation|PlayAnimation (Variables|Default|GetWeaponSkeletalMesh) "/Game/Items/Weapons/Bow/Animations/A_bow_3rd_draw_c2.A_bow_3rd_draw_c2" false))))

(event Custom|SignalSpecialSettleStart
  (if (Variables|Default|GetInThirdPerson)
    (Components|Animation|PlayAnimation (Variables|Default|GetWeaponSkeletalMesh) "/Game/Items/Weapons/Bow/Animations/A_bow_3rd_secondary_special_settle.A_bow_3rd_secondary_special_settle" false)
    (else
      (Components|Animation|PlayAnimation (Variables|Default|GetWeaponSkeletalMesh) "/Game/Items/Weapons/Bow/Animations/A_bow_1st_secondary_special_settle.A_bow_1st_secondary_special_settle" false))))

(event Custom|SpawnArrow
  (bind _owner (CallFunction|GetCharacterOwner))
  (if (not (Networking|IsServer))
    (bind _returnvalue (Utilities|GetDataTableRow "/Game/Items/ItemTable.ItemTable" (Utilities|String|StringToName (Utilities|String|ToString(Integer) (Class|GameItem|GetIntStat (Variables|Default|GetOwnerItem) "ActiveAmmunition"))) :!label _label)
      (:then
        (bind _object (Utilities|AsyncLoadAsset (.VisualStaticMesh (Utilities|Struct|BreakItemTableRow _returnvalue))))
        (bind _returnvalue_2 (Game|SpawnActorfromClass "/Game/Items/Weapons/Bow/BP_Visual_BowProjectileBase.BP_Visual_BowProjectileBase_C" (Transformation|GetSocketTransform (Variables|/Script/Engine.Character|GetMesh (CallFunction|GetCharacterOwner)) "Socket_Bow_Arrow" "RTS_World") "AlwaysSpawn" _owner true _object 0 false 0.0 0.0 0 "None" _owner))
        (Variables|Default|SetLoadedProjectile _returnvalue_2)
        (Networking|SetReplicates (Variables|Default|GetLoadedProjectile) false)
        (Transformation|AttachComponentToComponent (Variables|Default|GetLoadedProjectile) (Variables|/Script/Engine.Character|GetMesh (CallFunction|GetCharacterOwner)) "Socket_Bow_Arrow" "SnapToTarget" "SnapToTarget" "SnapToTarget" true)))
    (else
      (bind _isremote (Default|IsRemoteActor (CallFunction|GetCharacterOwner)))
      (if (not _isremote)
        (goto _label)))))

(event EventBeginPlay
  (|CallParentFunction)
  (Utilities|FlowControl|Sequence
    (:then_0
      (Utilities|FlowControl|Sequence
        (:then_0
          (bind _asis_in_third_person_interface (Utilities|Casting|CastToIsInThirdPersonInterface (Components|GetOwner)))
          (bind _returnvalue (Class|IsinThirdPersonInterface|GetIsinThirdPerson _asis_in_third_person_interface))
          (Variables|Default|SetInThirdPerson _returnvalue))
        (:then_1
          (bind _asab_human_male (Utilities|Casting|CastToAB_human_male (Components|SkeletalMesh|GetAnimInstance (Variables|/Script/Engine.Character|GetMesh (CallFunction|GetCharacterOwner)))))
          (Variables|Default|SetAnimBP _asab_human_male))))
    (:then_1
      ;[1 1 1] Basic String Draw
      (EventDispatchers|BindEventtoSignalPrimaryStringDraw (CallFunction|GetCharacterOwner) (delegate Custom|SignalPrimaryStringDraw)))
    (:then_2
      ;[1 1 1] Basic String Draw
      (EventDispatchers|BindEventtoSignalSecondaryStringDraw (CallFunction|GetCharacterOwner) (delegate Custom|SignalSecondaryStringDraw))
      (EventDispatchers|BindEventtoSignalSecondaryStringLoop (CallFunction|GetCharacterOwner) (delegate Custom|SignalSecondaryStringLoop))
      ;[1 1 1] Basic String Execute
      (EventDispatchers|AssignSignalBowStringExecute (CallFunction|GetCharacterOwner) (delegate Custom|SignalBowStringExecute))
      ;[1 1 1] Basic String Settle
      (EventDispatchers|BindEventtoSignalSecondaryStringSettle (CallFunction|GetCharacterOwner) (delegate Custom|SignalSecondaryStringSettle))
      (EventDispatchers|BindEventtoSignalSpecialSettleStart (CallFunction|GetCharacterOwner) (delegate Custom|SignalSpecialSettleStart)))
    (:then_3
      (EventDispatchers|BindEventtoSignalPickArrow (Variables|Default|GetAnimBP) (delegate Custom|SpawnArrow))
      (EventDispatchers|BindEventtoSignalAttackCollision (CallFunction|GetCharacterOwner) (EventDispatchers|CreateEvent :!event DestroyLoadedProjectile))
      (EventDispatchers|BindEventtoSignalBasicSettleEnd (Variables|Default|GetAnimBP) (EventDispatchers|CreateEvent :!event DestroyLoadedProjectile))
      (EventDispatchers|BindEventtoSignalSpecialSettleEnd (Variables|Default|GetAnimBP) (EventDispatchers|CreateEvent :!event DestroyLoadedProjectile))
      (EventDispatchers|BindEventtoOnCharacterSubstateChanged (CallFunction|GetCharacterOwner) (EventDispatchers|CreateEvent :!event OnExitCombatDestroyArrowProjectile)))))

(event EventEndPlay
  (params (EndPlayReason :type EEndPlayReason%20Enum :default "Destroyed"))
  (CallFunction|DestroyLoadedProjectile))

(fn ConstructionScript
  (|CallParentFunction))

(fn OnExitCombatDestroyArrowProjectile
  (params (Substate :type CharacterSubState%20Enum) (Entered :type Boolean))
  (if (and (Utilities|Enum|Equal(Enum) Substate "NewEnumerator21") (not Entered))
    (CallFunction|DestroyLoadedProjectile)))