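; BP_Shield_Weapon_Light is a shield weapon whose collision box is live only while attacking, which serves as blocking.
; Start and end attack toggle query-only collision, and IsShieldActive reads that state.
; Visual changes set the box's physical material from the weapon material, and breaking notifies an NPC owner via ShieldBroken.
; With combat debug logging enabled, Tick draws the blocking box in red.
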(event EventStartAttacking
  (params (AttackType :type SimpleAttack_AttackTypes%20Enum :default "NewEnumerator0"))
  (|CallParentFunction AttackType)
  (Collision|SetCollisionEnabled (Variables|Default|GetWeaponCollision) "QueryOnly")
  ;[0.62 0 0] For debugging blocking.
  (if (Class|LoggerLibrary|IsSuppressed "INFOL_INFO0" "Combat")
    (Actor|Tick|SetActorTickEnabled false)
    (else
      (Actor|Tick|SetActorTickEnabled true)
      (Variables|Default|SetActiveDebugEnabled true))))

(event EventTick
  (params (DeltaSeconds :type Float%20%28single-precision%29))
  (bind _weaponcollision (Variables|Default|GetWeaponCollision))
  ;[0.62 0 0] Debug Blocking
  (if (not (Class|LoggerLibrary|IsSuppressed "INFOL_INFO0" "Combat"))
    (if (Variables|Default|GetActiveDebugEnabled)
      (Rendering|Debug|DrawDebugBox (.Origin (Collision|GetComponentBounds _weaponcollision)) (Variables|/Script/Engine.BoxComponent|GetBoxExtent _weaponcollision) "(R=1.000000,G=0.000000,B=0.000000,A=1.000000)" (Transformation|GetWorldRotation _weaponcollision) 0.0 5.0))))

(event EventOnVisualsChanged
  (bind _value (Class|BaseWeaponInterface|GetWeaponMaterial(Message) self))
  (Class|PrimitiveComponent|SetPhysMaterialOverride (Variables|Default|GetWeaponCollision) (Class|MaterialInterface|GetPhysicalMaterial _value)))

(event EventBeginPlay
  (|CallParentFunction)
  (Collision|SetCollisionEnabled (Variables|Default|GetWeaponCollision) "NoCollision"))

(event EventEndAttacking
  (|CallParentFunction)
  (Collision|SetCollisionEnabled (Variables|Default|GetWeaponCollision) "NoCollision")
  (Variables|Default|SetActiveDebugEnabled false))

(event EventWeaponBroken
  (|CallParentFunction)
  (bind _asbp_npccharacter_interface (Utilities|Casting|CastToBP_NPCCharacterInterface (CallFunction|GetCharacterOwner)))
  (Default|ShieldBroken _asbp_npccharacter_interface))

(fn ConstructionScript
  (|CallParentFunction))

(fn IsShieldActive
  (return (Utilities|Enum|NotEqual(Enum) (Collision|GetCollisionEnabled (Variables|Default|GetWeaponCollision)) "NoCollision")))