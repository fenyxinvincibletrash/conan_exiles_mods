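; Buff component that greatly raises the owning character's Armor and NaturalArmor while active.
; On start it removes the Increase Rage buff through the character's BuffSystem component, then applies flat additive stat modifiers under the Buff ID.
; On clear it re-applies those modifiers with a zero value.
; Its description text instead reads "Armor reduced", with a value that ignores stack size.
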(event EventBeginPlay)

(event EventTick
  (params (DeltaSeconds :type Float%20%28single-precision%29)))

(event EventGameplayEffecttoApplyonBuffStart
  (bind _owningcharacter (Variables|Default|GetOwningCharacter))
  (Default|RemoveBuff (Utilities|Array|Get(acopy) (Actor|GetComponentsByClass _owningcharacter "/Game/Systems/Buffs/00_BP_AC_BuffSystem.00_BP_AC_BuffSystem_C")) "/Game/Mods/NewBosses/Weapons/BP_AC_Buff_Increase_Rage.BP_AC_Buff_Increase_Rage_C")
  (Class|ConanCharacter|AddFloatStatModifier _owningcharacter "Armor" "Buff" "Add" 3e+03 "Replace")
  (Class|ConanCharacter|AddFloatStatModifier _owningcharacter "NaturalArmor" "Buff" "Add" 3e+03 "Replace"))

(event EventGameplayEffecttoApplyonBuffCleared
  (bind _owningcharacter (Variables|Default|GetOwningCharacter))
  (Class|ConanCharacter|AddFloatStatModifier _owningcharacter "Armor" "Buff" "Add" 0.0 "Replace")
  (Class|ConanCharacter|AddFloatStatModifier _owningcharacter "NaturalArmor" "Buff" "Add" 0.0 "Replace"))

(fn GetEffectDescription
  (return (Utilities|Text|FormatText "Armor reduced by {ArmorReduction}%" (- 1.0 (* (Variables|Default|GetStackSize) 0.0)))))