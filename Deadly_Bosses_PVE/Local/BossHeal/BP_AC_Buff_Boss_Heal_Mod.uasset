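; Boss heal buff component for the Deadly Bosses PVE mod that sets up a heal over time on a BasePlayerChar.
; On start, it sizes each tick so that all ticks together total about a third of the character's full max health.
; The parent buff start runs only if no large healing potion buff is present; the server then ends any Hearty Meal and small healing potion buffs.
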(event EventStartBuff
  (params (BuffPotency :type Integer) (DamageCauser :type Actor%20Object%20Reference) (OwningCharacter :type Conan%20Character%20Object%20Reference) (Instigator :type Controller%20Object%20Reference))
  (bind _asbase_player_char (Utilities|Casting|CastToBasePlayerChar OwningCharacter))
  (Variables|Default|SetHealOverTimeValue (Math|Float|Truncate (/ (* (Class|ConanCharacter|GetIntStat _asbase_player_char "HealthMax" "Full") 0.33) (Math|Conversions|ToFloat(Integer) (Variables|/Game/Systems/Buffs/01_BP_AC_Buff_Master.01_BP_AC_Buff_Master_C|GetBuffTicks self)))))
  (if (not (> (Utilities|Array|Length (Actor|GetComponentsByClass _asbase_player_char "/Game/Systems/Buffs/Heal_OverTime/BP_AC_Buff_HealingPotion_Large.BP_AC_Buff_HealingPotion_Large_C")) 0))
    (|CallParentFunction BuffPotency DamageCauser OwningCharacter Instigator)
    (bind _asbase_player_char_2 (Utilities|Casting|CastToBasePlayerChar (Variables|Default|GetOwningCharacter)))
    (if (Networking|IsServer)
      (Default|EndBuff (Variables|/Game/Characters/BaseBPCombat.BaseBPCombat_C|Get00_BP_AC_BuffSystem _asbase_player_char_2) "/Game/Systems/Buffs/Heal_OverTime/BP_AC_Buff_Healing_HeartyMeal.BP_AC_Buff_Healing_HeartyMeal_C")
      (Default|EndBuff (Variables|/Game/Characters/BaseBPCombat.BaseBPCombat_C|Get00_BP_AC_BuffSystem _asbase_player_char_2) "/Game/Systems/Buffs/Heal_OverTime/BP_AC_Buff_HealingPotion_Small.BP_AC_Buff_HealingPotion_Small_C"))))